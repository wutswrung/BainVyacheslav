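; Bunker gate that opens automatically the first time anything overlaps its trigger Box.
; The overlap swaps two pairs of closed/open indicator planes, then plays a staged sequence of welcome, card and electric door sounds separated by delays.
; A Timeline then drives Lerps that slide the left and right doors apart along their relative Y axis.
; A DoOnce gates the sequence, and the graph has no closing logic.
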(event OnComponentBeginOverlap(Box)
  (params (OverlappedComponent :type Primitive%20Component%20Object%20Reference) (OtherActor :type Actor%20Object%20Reference) (OtherComp :type Primitive%20Component%20Object%20Reference) (OtherBodyIndex :type Integer) (bFromSweep :type Boolean) (SweepResult :type Hit%20Result%20Structure%20%28by%20ref%29))
  (bind _returnvalue (Transformation|GetActorLocation))
  (Utilities|FlowControl|DoOnce false
    (:Completed
      (Rendering|SetVisibility (Variables|Default|GetPlaneClosed) false false)
      (Rendering|SetVisibility (Variables|Default|GetPlaneOpem) true false)
      (Audio|PlaySoundatLocation "/Game/BainProject/Noise/NewNoises/Welcome.Welcome" _returnvalue "0, 0, 0" 1.0 1.0 0.0 0 0 0)
      (Utilities|FlowControl|Delay 1.0)
      (Audio|PlaySoundatLocation "/Game/BainProject/Noise/Door/doorOpen__online-audio-converter_com_.doorOpen__online-audio-converter_com_" _returnvalue "0, 0, 0" 1.0 1.0 0.0 0 0 0)
      (Audio|PlaySoundatLocation "/Game/BainProject/Noise/Door/OpenCard.OpenCard" _returnvalue "0, 0, 0" 1.0 1.0 0.0 0 0 0)
      (Utilities|FlowControl|Delay 1.0)
      (Audio|PlaySoundatLocation "/Game/BainProject/Noise/DverElektricheskaya.DverElektricheskaya" (Transformation|GetActorLocation) "0, 0, 0" 1.0 1.0 0.0 0 0 0)
      (Utilities|FlowControl|Delay 0.2)
      (bind _doortransform1 (Timeline|Timeline_0 Play)
        (:Update
          (Utilities|FlowControl|Sequence
            (:then_0
              (Transformation|SetRelativeLocation (Variables|Default|GetDoorLeft) (Math|Vector|MakeVector 2.0 (Math|Float|Lerp 138.0 3.5e+02 _doortransform1) -56.0) false false))
            (:then_1
              (Transformation|SetRelativeLocation (Variables|Default|GetDoorRight) (Math|Vector|MakeVector 23.0 (Math|Float|Lerp -129.0 -3.5e+02 _doortransform1) -56.0) false false))))))))

(fn ConstructionScript)