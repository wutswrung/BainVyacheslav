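; Bunker gate actor that slides open for a player holding the key card and otherwise sends them to find it.
; On box overlap, MainCharacter's KeyUp triggers a one-time opening: indicator planes swap, sounds play, then a timeline lerps both doors apart.
; Without it, denial sounds and timed text show; the first denial also displays widgets and updates the player's objective.
; An unconnected branch would change the South Gate card's item category.
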(event OnComponentBeginOverlap(Box)
  (params (OverlappedComponent :type Primitive%20Component%20Object%20Reference) (OtherActor :type Actor%20Object%20Reference) (OtherComp :type Primitive%20Component%20Object%20Reference) (OtherBodyIndex :type Integer) (bFromSweep :type Boolean) (SweepResult :type Hit%20Result%20Structure%20%28by%20ref%29))
  (bind _returnvalue (Transformation|GetActorLocation))
  (bind _textrender (Variables|Default|GetTextRender))
  (bind _asmain_character (Utilities|Casting|CastToMainCharacter OtherActor))
  (if (Variables|/Game/BainProject/Characters/MainCharacter.MainCharacter_C|GetKey%20Up _asmain_character)
    (Utilities|FlowControl|DoOnce false
      (:Completed
        (Rendering|SetVisibility (Variables|Default|GetPlaneClosed) false false)
        (Rendering|SetVisibility (Variables|Default|GetPlaneOpem) true false)
        (Audio|PlaySoundatLocation "/Game/BainProject/Noise/NewNoises/Welcome.Welcome" _returnvalue "0, 0, 0" 1.0 1.0 0.0 0 0 0)
        (Utilities|FlowControl|Delay 1.0)
        (Audio|PlaySoundatLocation "/Game/BainProject/Noise/Door/doorOpen__online-audio-converter_com_.doorOpen__online-audio-converter_com_" _returnvalue "0, 0, 0" 1.0 1.0 0.0 0 0 0)
        (Audio|PlaySoundatLocation "/Game/BainProject/Noise/Door/OpenCard.OpenCard" _returnvalue "0, 0, 0" 1.0 1.0 0.0 0 0 0)
        (Utilities|FlowControl|Delay 1.0)
        (Audio|PlaySoundatLocation "/Game/BainProject/Noise/DverElektricheskaya.DverElektricheskaya" (Transformation|GetActorLocation) "0, 0, 0" 1.0 1.0 0.0 0 0 0)
        (Utilities|FlowControl|Delay 0.2)
        (bind _doortransform1 (Timeline|Timeline_0 Play)
          (:Update
            (Utilities|FlowControl|Sequence
              (:then_0
                (Transformation|SetRelativeLocation (Variables|Default|GetDoorLeft) (Math|Vector|MakeVector 2.0 (Math|Float|Lerp 138.0 3.5e+02 _doortransform1) -56.0) false false))
              (:then_1
                (Transformation|SetRelativeLocation (Variables|Default|GetDoorRight) (Math|Vector|MakeVector 23.0 (Math|Float|Lerp -129.0 -3.5e+02 _doortransform1) -56.0) false false)))))))
    (else
      (Audio|PlaySoundatLocation "/Game/BainProject/Noise/Door/NoAccess__online-audio-converter_com_.NoAccess__online-audio-converter_com_" "0, 0, 0" "0, 0, 0" 1.0 1.0 0.0 0 0 0)
      (Audio|PlaySoundatLocation "/Game/BainProject/Noise/Door/AccessDenied.AccessDenied" _returnvalue "0, 0, 0" 1.0 1.0 0.0 0 0 0)
      (Utilities|FlowControl|Sequence
        (:then_0
          (Rendering|SetVisibility _textrender true false)
          (Utilities|FlowControl|Delay 3.0)
          (Rendering|SetVisibility _textrender false false))
        (:then_1
          (Utilities|FlowControl|DoOnce false
            (:Completed
              (bind _returnvalue_2 (UserInterface|CreateWidget "/Game/BainProject/UI_UX/Dialogues/NyjnaKlychKarta.NyjnaKlychKarta_C"))
              (bind _output_get (Variables|Default|SetNewVar_1 _returnvalue_2))
              (UserInterface|Viewport|AddtoViewport _output_get 0)
              (Utilities|FlowControl|Delay 4.0)
              (Widget|RemovefromParent _output_get)
              (Variables|/Game/BainProject/Characters/MainCharacter.MainCharacter_C|SetPlayerObjective _asmain_character "3. НАЙТИ КЛЮЧ КАРТУ")
              (Variables|/Game/BainProject/Characters/MainCharacter.MainCharacter_C|SetObjectiveDescription _asmain_character "ВОРОТА ЗАКРЫТЫ, НАДО НАЙТИ КЛЮЧ КАРТУ ДЕЖУРНОГО СЕРЖАНТА КИРКА, РЯДОМ С ЕГО ТРУПОМ ЛЕЖАЛ ЖУРНАЛ, ДУМАЮ В НЕМ НАПИСАНО КАК ОТКРЫТ ВОРОТА.")
              (Audio|PlaySound2D "/Game/BainProject/Noise/NewNoises/laser-scan_fjjawtv_.laser-scan_fjjawtv_" 1.0 1.0 0.0 0 0)
              (bind _returnvalue_3 (UserInterface|CreateWidget "/Game/BainProject/UI_UX/Menu/PROLOGUE/Uvedomlenie.Uvedomlenie_C"))
              (bind _output_get_2 (Variables|Default|SetNewVar_0 _returnvalue_3))
              (UserInterface|Viewport|AddtoViewport _output_get_2 0)
              (Utilities|FlowControl|Delay 4.0)
              (Widget|RemovefromParent _output_get_2))))))))

(fn ConstructionScript)