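; Ceiling ventilation Blueprint in the Bunker map that slides a vent mesh shut once the player's main character flags it as closed.
; Tick polls the character's VentClosed flag and fires the close event through a DoOnce, so it runs a single time.
; The event plays a 2D sound and a timeline that lerps the mesh's relative Y location to its closed position.
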(event Custom|VentilationClose
  (Audio|PlaySound2D "/Game/BainProject/Noise/kuhonnyiy-shkaf-zadvigaetsya-29119.kuhonnyiy-shkaf-zadvigaetsya-29119" 1.0 1.0 0.0 0 0)
  (bind _closevent (Timeline|VentClose Play)
    (:Update
      (Transformation|SetRelativeLocation (Variables|Default|GetStaticMesh1) (Math|Vector|MakeVector 0.0 (Math|Float|Lerp -147.0 0.0 _closevent) 0.0) false false))))

(event EventBeginPlay)

(event Collision|EventActorBeginOverlap
  (params (OtherActor :type Actor%20Object%20Reference)))

(event EventTick
  (params (DeltaSeconds :type Float%20%28single-precision%29))
  (bind _asmain_character (Utilities|Casting|CastToMainCharacter (Game|GetPlayerCharacter 0)))
  (if (Variables|/Game/BainProject/Characters/MainCharacter.MainCharacter_C|GetVentClosed _asmain_character)
    (Utilities|FlowControl|DoOnce false
      (:Completed
        (CallFunction|VentilationClose)))))

(fn ConstructionScript)