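; ItemPictureCosmos is an inventory item that displays a cosmos picture widget when used.
; On use it creates W_PictureCosmos with a reference to itself and adds it centered and auto-sized to the inventory main widget's canvas.
; OnRead removes that widget and destroys the item actor.
; Nodes for toggling the inventory widget and changing input mode are present but unconnected.
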(event Custom|OnRead
  (Widget|RemovefromParent (Variables|Default|GetPictCosmos))
  (Actor|DestroyActor))

(event EventBeginPlay
  (|CallParentFunction))

(event Collision|EventActorBeginOverlap
  (params (OtherActor :type Actor%20Object%20Reference))
  (|CallParentFunction OtherActor) ; This node is disabled and will not be called.\nDrag off pins to build functionality.
)

(event EventTick
  (params (DeltaSeconds :type Float%20%28single-precision%29))
  (|CallParentFunction DeltaSeconds) ; This node is disabled and will not be called.\nDrag off pins to build functionality.
)

(event EventEventonUsed
  (bind _returnvalue (UserInterface|CreateWidget "/Game/BainProject/InventorySystem/Widgets/W_PictureCosmos.W_PictureCosmos_C" 0 self))
  (bind _output_get (Variables|Default|SetPictCosmos _returnvalue))
  (bind _returnvalue_2 (Class|CanvasPanel|AddChildtoCanvas (Variables|/Game/BainProject/InventorySystem/Widgets/W_MainWidget.W_MainWidget_C|GetCanvasPanel_0 (Variables|/Game/BainProject/InventorySystem/Blueprints/BP_Inventory.BP_Inventory_C|GetMainWidget (Variables|Default|GetInventory))) _output_get))
  (Class|CanvasPanelSlot|SetAnchors _returnvalue_2 (Utilities|Struct|MakeAnchors "(X=0.500000,Y=0.500000)" "(X=0.500000,Y=0.500000)"))
  (Class|CanvasPanelSlot|SetAutoSize _returnvalue_2 true)
  (Class|CanvasPanelSlot|SetAlignment _returnvalue_2 "(X=0.500000,Y=0.500000)"))

(fn ConstructionScript
  (|CallParentFunction))