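; ItemSyrup is a healing inventory item that restores a fixed amount of HP to the player character when used.
; On use, if current HP in the player's StatusAC is below max, it adds the heal without clamping, plays a sound and removes one unit from the inventory.
; At full health it only plays a different sound, keeping the inventory entry.
; The actor destroys itself in both cases.
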(event EventBeginPlay
  (|CallParentFunction) ; This node is disabled and will not be called.\nDrag off pins to build functionality.
)

(event Collision|EventActorBeginOverlap
  (params (OtherActor :type Actor%20Object%20Reference))
  (|CallParentFunction OtherActor) ; This node is disabled and will not be called.\nDrag off pins to build functionality.
)

(event EventTick
  (params (DeltaSeconds :type Float%20%28single-precision%29))
  (|CallParentFunction DeltaSeconds) ; This node is disabled and will not be called.\nDrag off pins to build functionality.
)

(event EventEventonUsed
  (bind _returnvalue (Game|GetPlayerCharacter 0))
  (bind _asmain_character (Utilities|Casting|CastToMainCharacter _returnvalue))
  (bind _statusac (Variables|/Game/BainProject/Characters/MainCharacter.MainCharacter_C|GetStatusAC _asmain_character))
  (if (< (Variables|/Game/BainProject/Characters/StatusAC.StatusAC_C|GetCurrenHP _statusac) (Variables|/Game/BainProject/Characters/StatusAC.StatusAC_C|GetMaxHP _statusac))
    (Variables|/Game/BainProject/Characters/StatusAC.StatusAC_C|SetCurrenHP _statusac (+ (Variables|/Game/BainProject/Characters/StatusAC.StatusAC_C|GetCurrenHP _statusac) 2e+01))
    (Audio|PlaySound2D "/Game/BainProject/Noise/UsefullThings/Glotok.Glotok" 1.0 1.0 0.0 0 0)
    (Default|-RemoveItematIndex (Variables|Default|GetInventory) (Variables|Default|GetIndex) 1 false)
    (Actor|DestroyActor)
    (else
      (Audio|PlaySound2D "/Game/BainProject/Noise/UsefullThings/box-cardboard-close-lid_zkrf-v4o.box-cardboard-close-lid_zkrf-v4o" 1.0 1.0 0.0 0 0)
      (Actor|DestroyActor))))

(fn ConstructionScript
  (|CallParentFunction))