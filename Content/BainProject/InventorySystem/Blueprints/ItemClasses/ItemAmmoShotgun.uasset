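; Shotgun ammo item for the inventory system that loads one shell into the player's active weapon when used.
; On use, if the weapon's shotgun ammo count is at most five, it removes one item from the inventory, increments the count and plays an insert sound.
; Otherwise it only plays a pickup sound, and both branches destroy the actor.
; BeginPlay and overlap defer to the parent class.
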(event EventBeginPlay
  (|CallParentFunction))

(event Collision|EventActorBeginOverlap
  (params (OtherActor :type Actor%20Object%20Reference))
  (|CallParentFunction OtherActor))

(event EventTick
  (params (DeltaSeconds :type Float%20%28single-precision%29))
  (|CallParentFunction DeltaSeconds) ; This node is disabled and will not be called.\nDrag off pins to build functionality.
)

(event EventEventonUsed
  (bind _returnvalue (Game|GetPlayerCharacter 0))
  (bind _asmain_character (Utilities|Casting|CastToMainCharacter _returnvalue))
  (bind _activeweapon (Variables|/Game/BainProject/Characters/MainCharacter.MainCharacter_C|GetActiveWeapon _asmain_character))
  (bind _ammoac1 (Variables|/Game/BainProject/Weapon/WeaponBase.WeaponBase_C|GetAmmoAC1 _activeweapon))
  (if (<= (Variables|/Game/BainProject/Weapon/AmmoAC1.AmmoAC1_C|GetCurrentAmmoShotgun _ammoac1) 5)
    (Default|-RemoveItematIndex (Variables|Default|GetInventory) (Variables|Default|GetIndex) 1 false)
    (Variables|/Game/BainProject/Weapon/AmmoAC1.AmmoAC1_C|SetCurrentAmmoShotgun _ammoac1 (+ (Variables|/Game/BainProject/Weapon/AmmoAC1.AmmoAC1_C|GetCurrentAmmoShotgun _ammoac1) 1))
    (Audio|PlaySound2D "/Game/BainProject/Weapon/Shooting/Reload_Insert.Reload_Insert" 1.0 1.0 0.0 0 0)
    (Actor|DestroyActor)
    (else
      (Audio|PlaySound2D "/Game/BainProject/Noise/UsefullThings/ammopick.ammopick" 1.0 1.0 0.0 0 0)
      (Actor|DestroyActor))))

(fn ConstructionScript
  (|CallParentFunction))