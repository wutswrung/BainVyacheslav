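; Ammo item for the inventory system that adds reserve rounds to the player character's active weapon when used.
; Its used event reads the AmmoAC1 component on that weapon and adds a fixed 12 to AllAmmo, but only if CurrentAmmo is zero.
; With any CurrentAmmo left the event does nothing, and the graph itself neither reloads nor removes the item.
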(event EventBeginPlay
  (|CallParentFunction) ; This node is disabled and will not be called.\nDrag off pins to build functionality.
)

(event Collision|EventActorBeginOverlap
  (params (OtherActor :type Actor%20Object%20Reference))
  (|CallParentFunction OtherActor) ; This node is disabled and will not be called.\nDrag off pins to build functionality.
)

(event EventTick
  (params (DeltaSeconds :type Float%20%28single-precision%29))
  (|CallParentFunction DeltaSeconds) ; This node is disabled and will not be called.\nDrag off pins to build functionality.
)

(event EventEventonUsed
  (bind _returnvalue (Game|GetPlayerCharacter 0))
  (bind _asmain_character (Utilities|Casting|CastToMainCharacter _returnvalue))
  (bind _activeweapon (Variables|/Game/BainProject/Characters/MainCharacter.MainCharacter_C|GetActiveWeapon _asmain_character))
  (bind _ammoac1 (Variables|/Game/BainProject/Weapon/WeaponBase.WeaponBase_C|GetAmmoAC1 _activeweapon))
  (if (== (Variables|/Game/BainProject/Weapon/AmmoAC1.AmmoAC1_C|GetCurrentAmmo _ammoac1) 0)
    (Variables|/Game/BainProject/Weapon/AmmoAC1.AmmoAC1_C|SetAllAmmo _ammoac1 (+ (Variables|/Game/BainProject/Weapon/AmmoAC1.AmmoAC1_C|GetAllAmmo _ammoac1) 12))))

(fn ConstructionScript
  (|CallParentFunction))