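; World pickup actor for an inventory item, taking its mesh, scale, interaction radius and prompt name from the ItemClass defaults.
; Sphere overlaps maintain the character's NearbyPickUpActors queue, so only the first entry shows its "[E]" prompt.
; OnPickUp plays a sound and adds the item to the inventory, keeping any remainder and otherwise destroying itself, even on failure.
; Picking up the south gate card also sets the player's KeyUp flag.
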(event OnComponentBeginOverlap(Sphere)
  (params (OverlappedComponent :type Primitive%20Component%20Object%20Reference) (OtherActor :type Actor%20Object%20Reference) (OtherComp :type Primitive%20Component%20Object%20Reference) (OtherBodyIndex :type Integer) (bFromSweep :type Boolean) (SweepResult :type Hit%20Result%20Structure%20%28by%20ref%29))
  (bind _asmain_character (Utilities|Casting|CastToMainCharacter OtherActor))
  (if (> (Utilities|Array|Length (Variables|/Game/BainProject/Characters/MainCharacter.MainCharacter_C|GetNearbyPickUpActors _asmain_character)) 0)
    (Utilities|Array|Add (Variables|/Game/BainProject/Characters/MainCharacter.MainCharacter_C|GetNearbyPickUpActors _asmain_character) self)
    (else
      (Rendering|SetVisibility (Variables|Default|GetPickUpText) true false)
      (Utilities|Array|Add (Variables|/Game/BainProject/Characters/MainCharacter.MainCharacter_C|GetNearbyPickUpActors _asmain_character) self))))

(event OnComponentEndOverlap(Sphere)
  (params (OverlappedComponent :type Primitive%20Component%20Object%20Reference) (OtherActor :type Actor%20Object%20Reference) (OtherComp :type Primitive%20Component%20Object%20Reference) (OtherBodyIndex :type Integer))
  (bind _asmain_character (Utilities|Casting|CastToMainCharacter OtherActor))
  (if (and (Utilities|IsValid (Utilities|Array|Get(acopy) (Variables|/Game/BainProject/Characters/MainCharacter.MainCharacter_C|GetNearbyPickUpActors _asmain_character))) (== (Utilities|Array|Get(acopy) (Variables|/Game/BainProject/Characters/MainCharacter.MainCharacter_C|GetNearbyPickUpActors _asmain_character)) self))
    (Rendering|SetVisibility (Variables|Default|GetPickUpText) false false)
    (Utilities|Array|RemoveItem (Variables|/Game/BainProject/Characters/MainCharacter.MainCharacter_C|GetNearbyPickUpActors _asmain_character) self)
    (Utilities|IsValid (Utilities|Array|Get(acopy) (Variables|/Game/BainProject/Characters/MainCharacter.MainCharacter_C|GetNearbyPickUpActors _asmain_character))
      (:Is%20Valid
        (Rendering|SetVisibility (Variables|BP_PickUpActor_C|GetPickUpText (Utilities|Array|Get(acopy) (Variables|/Game/BainProject/Characters/MainCharacter.MainCharacter_C|GetNearbyPickUpActors _asmain_character))) true false)))
    (else
      ;[1 1 1] Если вышли из радиуса, из массива нужно удалить данный ITEM
      (Utilities|Array|RemoveItem (Variables|/Game/BainProject/Characters/MainCharacter.MainCharacter_C|GetNearbyPickUpActors _asmain_character) self))))

(event Custom|OnPickUp
  (params (MainChar :type Main%20Character%20Object%20Reference))
  (bind _inventoryref (Variables|/Game/BainProject/Characters/MainCharacter.MainCharacter_C|GetInventoryRef MainChar))
  (bind _nearbypickupactors (Variables|/Game/BainProject/Characters/MainCharacter.MainCharacter_C|GetNearbyPickUpActors MainChar))
  (bind _output (Utilities|Array|Get(acopy) _nearbypickupactors))
  (Audio|PlaySound2D "/Game/BainProject/Noise/UsefullThings/box-cardboard-close-lid_zkrf-v4o.box-cardboard-close-lid_zkrf-v4o" 1.0 1.0 0.0 0 0)
  (Utilities|IsValid _inventoryref
    (:Is%20Valid
      (if (== (Variables|Default|GetItem%20Class) "/Game/BainProject/InventorySystem/Blueprints/ItemClasses/ItemCardSouthGate.ItemCardSouthGate_C")
        (Variables|/Game/BainProject/Characters/MainCharacter.MainCharacter_C|SetKey%20Up (.AsMain%20Character (Utilities|Casting|CastToMainCharacter (Game|GetPlayerCharacter 0))) true))
      (bind (_success2_ _rest2) (Default|-AddItem _inventoryref (Variables|Default|GetItem%20Class) (Variables|Default|GetAmount)))
      (if _success2_
        (if (> _rest2 0)
          (Variables|Default|SetAmount _rest2)
          (CallFunction|-UpdateText)
          (else
            (Actor|DestroyActor)))
        (else
          (Utilities|Array|RemoveItem _nearbypickupactors self)
          (Utilities|IsValid _output
            (:Is%20Valid
              (Rendering|SetVisibility (Variables|BP_PickUpActor_C|GetPickUpText _output) true false)
              (Actor|DestroyActor))
            (:Is%20Not%20Valid
              (Actor|DestroyActor))))))))

(event EventBeginPlay
  (CallFunction|-UpdateText))

(event Collision|EventActorBeginOverlap
  (params (OtherActor :type Actor%20Object%20Reference)))

(event EventTick
  (params (DeltaSeconds :type Float%20%28single-precision%29)))

(fn ConstructionScript
  (bind _item_class (Variables|Default|GetItem%20Class))
  (bind _staticmesh (Variables|Default|GetStaticMesh))
  (bind _iteminfo (Utilities|GetClassDefaults _item_class))
  (bind (_name _description _icon _canbeused _usetext _canbestacked _category _pickupmesh _meshscale _interactradius) (Utilities|Struct|Breaks_ItemInfo _iteminfo))
  (if (Utilities|IsValidClass _item_class)
    (Components|StaticMesh|SetStaticMesh _staticmesh _pickupmesh)
    (Variables|Default|SetOriginalMaterial (Rendering|Material|GetMaterial _staticmesh 0))
    (Transformation|SetRelativeScale3D _staticmesh _meshscale)
    (Components|Sphere|SetSphereRadius (Variables|Default|GetSphere) _interactradius false)))

(fn -OnUnhovered
  (Rendering|Material|SetMaterial (Variables|Default|GetStaticMesh) 0 (Variables|Default|GetOriginalMaterial)))

(fn -UpdateText
  (bind _asw_pick_up_text (Utilities|Casting|CastToW_PickUpText (UserInterface|GetUserWidgetObject (Variables|Default|GetPickUpText))))
  (Rendering|Components|TextRender|SetText (Variables|/Game/BainProject/InventorySystem/Widgets/W_PickUpText.W_PickUpText_C|GetNameText _asw_pick_up_text) (Utilities|Text|FormatText "{name} [E]" (.Name (Utilities|Struct|Breaks_ItemInfo (.ItemInfo (Utilities|GetClassDefaults (Variables|Default|GetItem%20Class))))))))