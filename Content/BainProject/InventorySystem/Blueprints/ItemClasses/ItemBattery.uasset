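; Battery inventory item that recharges the main character's PlayerBattery when used.
; On use it casts the player character and adds a fixed charge if below full, or plays a denial sound otherwise.
; Only when the addition overflows does it clamp the charge, set BatteryUp, play a sound, remove one item from the inventory and destroy itself; smaller top-ups leave the item in place.
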(event EventBeginPlay
  (|CallParentFunction) ; This node is disabled and will not be called.\nDrag off pins to build functionality.
)

(event Collision|EventActorBeginOverlap
  (params (OtherActor :type Actor%20Object%20Reference))
  (|CallParentFunction OtherActor) ; This node is disabled and will not be called.\nDrag off pins to build functionality.
)

(event EventTick
  (params (DeltaSeconds :type Float%20%28single-precision%29))
  (|CallParentFunction DeltaSeconds) ; This node is disabled and will not be called.\nDrag off pins to build functionality.
)

(event EventEventonUsed
  (bind _asmain_character (Utilities|Casting|CastToMainCharacter (Game|GetPlayerCharacter 0)))
  (if (< (Variables|/Game/BainProject/Characters/MainCharacter.MainCharacter_C|GetPlayerBattery _asmain_character) 100)
    ;[1 1 1] Добавление опр кол заряда
    (bind _output_get (Variables|/Game/BainProject/Characters/MainCharacter.MainCharacter_C|SetPlayerBattery _asmain_character (+ (Variables|/Game/BainProject/Characters/MainCharacter.MainCharacter_C|GetPlayerBattery _asmain_character) 50)))
    ;[1 1 1] Ограничение заряда
    (if (> _output_get 100)
      (Variables|/Game/BainProject/Characters/MainCharacter.MainCharacter_C|SetPlayerBattery _asmain_character 100)
      (Variables|/Game/BainProject/Characters/MainCharacter.MainCharacter_C|SetBattery%20Up _asmain_character true)
      (Audio|PlaySound2D "/Game/BainProject/Noise/UsefullThings/flashlight-no-batteries-set-down_gjkknvvu.flashlight-no-batteries-set-down_gjkknvvu" 1.0 1.0 0.0 0 0)
      (Default|-RemoveItematIndex (Variables|Default|GetInventory) (Variables|Default|GetIndex) 1)
      (Actor|DestroyActor))
    (else
      (Audio|PlaySound2D "/Game/BainProject/Noise/Door/NoAccess__online-audio-converter_com_.NoAccess__online-audio-converter_com_" 1.0 1.0 0.0 0 0))))

(fn ConstructionScript
  (|CallParentFunction))