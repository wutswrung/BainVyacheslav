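; Inventory item for the Rita and Doomer photo, which the player views full widget-style and which is consumed afterwards.
; On use, it disables the inventory widget, adds a W_PhotoRitaAndDoomer centered on the main canvas and switches input to UI only.
; The widget receives the item through its PorterJournal pin.
; OnRead re-enables the inventory, removes the widget, restores game-and-UI input and destroys the actor.
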(event Custom|OnRead
  (Widget|SetIsEnabled (Variables|/Game/BainProject/InventorySystem/Widgets/W_MainWidget.W_MainWidget_C|GetInventoryWidget (Variables|/Game/BainProject/InventorySystem/Blueprints/BP_Inventory.BP_Inventory_C|GetMainWidget (Variables|Default|GetInventory))) true)
  (Widget|RemovefromParent (stale EventEventonUsed _output_get))
  (Input|SetInputModeGameandUI (Game|GetPlayerController 0) (stale EventEventonUsed _output_get) "DoNotLock" true)
  (Actor|DestroyActor))

(event EventBeginPlay
  (|CallParentFunction))

(event Collision|EventActorBeginOverlap
  (params (OtherActor :type Actor%20Object%20Reference))
  (|CallParentFunction OtherActor) ; This node is disabled and will not be called.\nDrag off pins to build functionality.
)

(event EventTick
  (params (DeltaSeconds :type Float%20%28single-precision%29))
  (|CallParentFunction DeltaSeconds) ; This node is disabled and will not be called.\nDrag off pins to build functionality.
)

(event EventEventonUsed
  (Widget|SetIsEnabled (Variables|/Game/BainProject/InventorySystem/Widgets/W_MainWidget.W_MainWidget_C|GetInventoryWidget (Variables|/Game/BainProject/InventorySystem/Blueprints/BP_Inventory.BP_Inventory_C|GetMainWidget (Variables|Default|GetInventory))) false)
  (bind _returnvalue (UserInterface|CreateWidget "/Game/BainProject/InventorySystem/Widgets/W_PhotoRitaAndDoomer.W_PhotoRitaAndDoomer_C" 0 self))
  (bind _output_get (Variables|Default|SetPhototW _returnvalue))
  (bind _returnvalue_2 (Class|CanvasPanel|AddChildtoCanvas (Variables|/Game/BainProject/InventorySystem/Widgets/W_MainWidget.W_MainWidget_C|GetCanvasPanel_0 (Variables|/Game/BainProject/InventorySystem/Blueprints/BP_Inventory.BP_Inventory_C|GetMainWidget (Variables|Default|GetInventory))) _output_get))
  (Class|CanvasPanelSlot|SetAnchors _returnvalue_2 (Utilities|Struct|MakeAnchors "(X=0.500000,Y=0.500000)" "(X=0.500000,Y=0.500000)"))
  (Class|CanvasPanelSlot|SetAutoSize _returnvalue_2 true)
  (Class|CanvasPanelSlot|SetAlignment _returnvalue_2 "(X=0.500000,Y=0.500000)")
  (Input|SetInputModeUIOnly (Game|GetPlayerController 0) _output_get "DoNotLock"))

(fn ConstructionScript
  (|CallParentFunction))