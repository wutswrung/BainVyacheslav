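; ItemRele is a relay inventory item that the player uses at an electrical panel linked to the safe armor room.
; Its used event acts only while the MainCharacter's SafeArmorRoomInteract flag marks the player as inside the panel's collision.
; It then hides the inventory, plays a sound, sets SafeArmorRoomCardUsed on the character, removes one item from the inventory and destroys itself.
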(event EventBeginPlay)

(event Collision|EventActorBeginOverlap
  (params (OtherActor :type Actor%20Object%20Reference)))

(event EventTick
  (params (DeltaSeconds :type Float%20%28single-precision%29)))

(event EventEventonUsed
  (bind _returnvalue (Game|GetPlayerCharacter 0))
  (bind _asmain_character (Utilities|Casting|CastToMainCharacter _returnvalue))
  ;[1 1 1] Скрываем инвентарь после нажатия на ItemRele в инвентаре, если он вне коллизии щитка
  (if (Variables|/Game/BainProject/Characters/MainCharacter.MainCharacter_C|GetSafeArmorRoomInteract _asmain_character)
    (Default|-HideInventory (Variables|/Game/BainProject/Characters/MainCharacter.MainCharacter_C|GetInventoryRef _asmain_character))
    (Audio|PlaySound2D "/Game/BainProject/Noise/UsefullThings/flashlight-pick-up-wood_m1tjnveu.flashlight-pick-up-wood_m1tjnveu" 1.0 1.0 0.0 "/Game/BainProject/Weapon/Shooting/NewSoundConcurrency.NewSoundConcurrency" 0)
    ;[1 1 1] Реле использовано и удаление предмета из инвентаря
    (Variables|/Game/BainProject/Characters/MainCharacter.MainCharacter_C|SetSafeArmorRoomCardUsed _asmain_character true)
    (Default|-RemoveItematIndex (Variables|Default|GetInventory) (Variables|Default|GetIndex) 1 false)
    (Actor|DestroyActor)))

(fn ConstructionScript
  (|CallParentFunction))