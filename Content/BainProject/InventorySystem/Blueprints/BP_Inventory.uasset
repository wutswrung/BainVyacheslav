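; Inventory actor that stores item class and amount in a fixed slot array and creates the main HUD widget displaying it.
; Functions add items by recursively filling stacks, swap, split, merge and remove them, refreshing changed slot widgets and optionally queuing obtained-item messages.
; Using an item spawns its class and triggers its use event.
; Drops spawn pickups ahead of the character, or at it when traces are blocked; the rotating-search step is unwired.
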(event Custom|UpdateSlotAtIndex
  (params (Index :type Integer))
  (Default|UpdateSlot (Utilities|Array|Get(acopy) (Variables|/Game/BainProject/InventorySystem/Widgets/W_Inventory.W_Inventory_C|GetSlotsWidgets (Variables|Default|GetInventory%20Widget)) Index)))

(event Custom|UseItemAtIndex
  (params (Index :type Integer))
  (bind _slots (Variables|Default|GetSlots))
  (bind _output (Utilities|Array|Get(acopy) _slots Index))
  (bind _itemclass (Utilities|Struct|Breaks_InventorySlot _output))
  (if (Utilities|IsValidClass _itemclass)
    (bind _returnvalue (Game|SpawnActorfromClass _itemclass (Math|Transform|MakeTransform "0, 0, 0" "0, 0, 0" "1,1,1") "AlwaysSpawn" 0 self Index 0))
    (Default|EventonUsed _returnvalue)))

(event EventBeginPlay
  ;[1 1 1] Зазмер относительно того кол-ва слотов, которое мы выделяем под инвентарь
  (Utilities|Array|Resize (Variables|Default|GetSlots) (Variables|Default|GetAmountOfSlots))
  (bind _returnvalue (UserInterface|CreateWidget "/Game/BainProject/InventorySystem/Widgets/W_MainWidget.W_MainWidget_C" 0 self (Variables|Default|GetSlots%20Per%20Row) (Variables|Default|GetObtainedVisibleDuration)))
  (bind _output_get (Variables|Default|SetMainWidget _returnvalue))
  (Variables|Default|SetInventory%20Widget (Variables|/Game/BainProject/InventorySystem/Widgets/W_MainWidget.W_MainWidget_C|GetInventoryWidget _output_get))
  (UserInterface|Viewport|AddtoViewport (Variables|Default|GetMainWidget) 0)
  (if (not (Variables|Default|GetShowObtainedMessage?))
    (Widget|RemovefromParent (Variables|/Game/BainProject/InventorySystem/Widgets/W_MainWidget.W_MainWidget_C|GetObtainedItemBorder (Variables|Default|GetMainWidget)))))

(fn ConstructionScript)

(fn -IsSlotEmpty?
  (params (Index :type Integer))
  (return (not (Utilities|IsValidClass (.ItemClass (Utilities|Struct|Breaks_InventorySlot (Utilities|Array|Get(acopy) (Variables|Default|GetSlots) Index)))))))

(fn -GetItemInfoatIndex
  (params (Index :type Integer))
  (bind _slots (Variables|Default|GetSlots))
  (bind _output (Utilities|Array|Get(acopy) _slots Index))
  (bind (_itemclass _amount) (Utilities|Struct|Breaks_InventorySlot _output))
  (if (Utilities|IsValidClass _itemclass)
    (return false (.ItemInfo (Utilities|GetClassDefaults _itemclass)) _amount)
    (else
      (return true "" 0))))

(fn -SearchEmptySlot
  ;[1 1 1] Выйти, если мы нашли пустой слот
  (bind (_array_element _array_index) (Utilities|Array|ForEachLoopwithBreak (Variables|Default|GetSlots) :!label _label)
    (:LoopBody
      (if (not (Utilities|IsValidClass (.ItemClass (Utilities|Struct|Breaks_InventorySlot _array_element))))
        (LocalVariables|SetLocalBool true)
        (LocalVariables|SetLocalIndex _array_index)
        (goto _label Break)))
    (:Completed
      (return (LocalVariables|GetLocalBool) (LocalVariables|GetLocalIndex)))))

(fn -SearchFreeStack
  (params (ItemClass :type BP%20Master%20Item%20Class%20Reference))
  (bind (_array_element _array_index) (Utilities|Array|ForEachLoopwithBreak (Variables|Default|GetSlots) :!label _label)
    (:LoopBody
      (if (Utilities|IsValidClass (.ItemClass (Utilities|Struct|Breaks_InventorySlot _array_element)))
        (if (and (== (.ItemClass (Utilities|Struct|Breaks_InventorySlot _array_element)) ItemClass) (< (.Amount (Utilities|Struct|Breaks_InventorySlot _array_element)) (Variables|Default|GetMaxStackSize)))
          (LocalVariables|SetLocalBool true)
          (LocalVariables|SetLocalIndex _array_index)
          (goto _label Break))))
    (:Completed
      (return (LocalVariables|GetLocalBool) (LocalVariables|GetLocalIndex)))))

(fn -AddItem
  (params (ItemClass :type BP%20Master%20Item%20Class%20Reference) (Amount :type Integer))
  (if (Variables|Default|GetShowObtainedMessage?)
    (bind (_success_ _rest) (CallFunction|-AddItem(Internal) ItemClass Amount))
    (if _success_
      (CallFunction|-ShowObtainedItem ItemClass (- Amount _rest))
      (return true _rest)
      (else
        (return true _rest)))
    (else
      (bind (_success__2 _rest_2) (CallFunction|-AddItem(Internal) ItemClass Amount))
      (return _success__2 _rest_2))))

(fn -GetAmountatIndex
  (params (Index :type Integer))
  (return (.Amount (Utilities|Struct|Breaks_InventorySlot (Utilities|Array|Get(acopy) (Variables|Default|GetSlots) Index)))))

(fn -RemoveItematIndex
  (params (Index :type Integer) (Amount :type Integer) (IsSpawn? :type Boolean))
  (bind _slots (Variables|Default|GetSlots))
  ;[1 1 1] Удаление эл-та из ячейки
  (LocalVariables|SetLocalIndex Index)
  (LocalVariables|SetLocalAmount Amount)
  (if (and (not (CallFunction|-IsSlotEmpty? (LocalVariables|GetLocalIndex))) (> (LocalVariables|GetLocalAmount) 0))
    (LocalVariables|SetLocal_SpawnItem (Utilities|Array|Get(acopy) _slots (LocalVariables|GetLocalIndex)))
    (if (>= (LocalVariables|GetLocalAmount) (CallFunction|-GetAmountatIndex (LocalVariables|GetLocalIndex)))
      ;;[1 1 1] Проверка каждого слота
      (Utilities|Array|SetArrayElem (Variables|Default|GetSlots) (LocalVariables|GetLocalIndex) (Utilities|Struct|Makes_InventorySlot 0 0))
      ;;[1 1 1] Отобразить изменения в ячейке
      (CallFunction|UpdateSlotatIndex (LocalVariables|GetLocalIndex))
      (else
        ;;[1 1 1] Уменьшили кол-во в определенном Item
        (Utilities|Array|SetArrayElem _slots (LocalVariables|GetLocalIndex) (Utilities|Struct|Makes_InventorySlot (.itemclass (Utilities|Array|Get(acopy) _slots (LocalVariables|GetLocalIndex))) (- (.amount (Utilities|Array|Get(acopy) _slots (LocalVariables|GetLocalIndex))) (LocalVariables|GetLocalAmount))))
        ;;;[1 1 1] Отобразить изменения в ячейке
        (CallFunction|UpdateSlotatIndex (LocalVariables|GetLocalIndex))))
    (if IsSpawn?
      (CallFunction|-SpawnItemsClassinWorld (.ItemClass (Utilities|Struct|Breaks_InventorySlot (LocalVariables|GetLocal_SpawnItem))) (LocalVariables|GetLocalAmount))
      (return true)
      (else
        (return true)))
    (else
      (return false))))

(fn -SwapSlots
  (params (Index1 :type Integer) (Index2 :type Integer))
  (bind _slots (Variables|Default|GetSlots))
  (bind _slots_2 (Variables|Default|GetSlots))
  (bind _returnvalue (Utilities|Array|LastIndex _slots))
  ;[1 1 1] Функция замены ячеек
  (LocalVariables|SetLocalIndex1 Index1)
  (LocalVariables|SetLocalIndex2 Index2)
  (if (or (> (LocalVariables|GetLocalIndex1) _returnvalue) (> (LocalVariables|GetLocalIndex2) _returnvalue))
    (return false)
    (else
      (LocalVariables|SetLocalSlot2 (Utilities|Array|Get(acopy) (Variables|Default|GetSlots) (LocalVariables|GetLocalIndex2)))
      (Utilities|Array|SetArrayElem _slots_2 (LocalVariables|GetLocalIndex2) (Utilities|Array|Get(acopy) _slots_2 (LocalVariables|GetLocalIndex1)))
      (Utilities|Array|SetArrayElem (Variables|Default|GetSlots) (LocalVariables|GetLocalIndex1) (LocalVariables|GetLocalSlot2))
      (CallFunction|UpdateSlotatIndex (LocalVariables|GetLocalIndex1))
      (CallFunction|UpdateSlotatIndex (LocalVariables|GetLocalIndex2))
      (return true))))

(fn -SplitStack
  (params (StackIndex :type Integer) (Amount :type Integer))
  (bind _slots (Variables|Default|GetSlots))
  (bind _slots_2 (Variables|Default|GetSlots))
  ;[1 1 1] Разделять предметы, которые стакаются на разные кол-ва
  (LocalVariables|SetLocalStackIndex StackIndex)
  (LocalVariables|SetLocalAmount Amount)
  (if (CallFunction|-IsSlotEmpty? (LocalVariables|GetLocalStackIndex))
    (return false)
    (elif (and (.CanBeStacked (Utilities|Struct|Breaks_ItemInfo (.ItemInfo (CallFunction|-GetItemInfoatIndex (LocalVariables|GetLocalStackIndex))))) (> (.Amount (CallFunction|-GetItemInfoatIndex (LocalVariables|GetLocalStackIndex))) (LocalVariables|GetLocalAmount)))
      (bind (_success_ _index) (CallFunction|-SearchEmptySlot))
      (if _success_
        (LocalVariables|SetLocalFoundIndex _index)
        (Utilities|Array|SetArrayElem _slots_2 (LocalVariables|GetLocalStackIndex) (Utilities|Struct|Makes_InventorySlot (.itemclass (Utilities|Array|Get(acopy) _slots_2 (LocalVariables|GetLocalStackIndex))) (- (.amount (Utilities|Array|Get(acopy) _slots_2 (LocalVariables|GetLocalStackIndex))) (LocalVariables|GetLocalAmount))))
        (Utilities|Array|SetArrayElem _slots (LocalVariables|GetLocalFoundIndex) (Utilities|Struct|Makes_InventorySlot (.itemclass (Utilities|Array|Get(acopy) _slots (LocalVariables|GetLocalStackIndex))) (LocalVariables|GetLocalAmount)))
        ;;[1 1 1] Меняем значения
        (CallFunction|UpdateSlotatIndex (LocalVariables|GetLocalStackIndex))
        (CallFunction|UpdateSlotatIndex (LocalVariables|GetLocalFoundIndex))
        (return true)
        (else
          (return false)))
      (else
        (return false)))))

(fn -ShowInventory
  (bind _mainwidget (Variables|Default|GetMainWidget))
  (UserInterface|Animation|PlayAnimation _mainwidget (Variables|/Game/BainProject/InventorySystem/Widgets/W_MainWidget.W_MainWidget_C|GetWithJournal _mainwidget) 0.0 1 "Forward" 1.0 false)
  (Widget|SetVisibility (Variables|Default|GetInventory%20Widget) "Visible")
  (Variables|Default|SetisVisible? true)
  (Widget|SetIsEnabled (Variables|Default|GetInventory%20Widget) true)
  (return))

(fn -HideInventory
  (Widget|SetVisibility (Variables|Default|GetInventory%20Widget) "Hidden")
  (Variables|Default|SetisVisible? false)
  (Widget|SetIsEnabled (Variables|Default|GetInventory%20Widget) false)
  (Widget|SetVisibility (Variables|/Game/BainProject/InventorySystem/Widgets/W_MainWidget.W_MainWidget_C|GetDropWidget (Variables|Default|GetMainWidget)) "Hidden")
  (Widget|SetIsEnabled (Variables|/Game/BainProject/InventorySystem/Widgets/W_Inventory.W_Inventory_C|GetSlotPanel (Variables|Default|GetInventory%20Widget)) true)
  (return))

(fn -AddtoIndex
  (params (FromIndex :type Integer) (ToIndex :type Integer))
  (LocalVariables|SetLocalFrom FromIndex)
  (LocalVariables|SetLocalTo ToIndex)
  (if (Math|Boolean|ANDBoolean (== (.itemclass (Utilities|Array|Get(acopy) (Variables|Default|GetSlots) (LocalVariables|GetLocalFrom))) (.itemclass (Utilities|Array|Get(acopy) (Variables|Default|GetSlots) (LocalVariables|GetLocalTo)))) (< (.amount (Utilities|Array|Get(acopy) (Variables|Default|GetSlots) (LocalVariables|GetLocalTo))) (Variables|Default|GetMaxStackSize)) (.CanBeStacked (Utilities|Struct|Breaks_ItemInfo (.ItemInfo (CallFunction|-GetItemInfoatIndex (LocalVariables|GetLocalFrom))))))
    (LocalVariables|SetLocalClass (.itemclass (Utilities|Array|Get(acopy) (Variables|Default|GetSlots) (LocalVariables|GetLocalFrom))))
    ;[1 1 1] Суммировали значени, записали в LocalTo
    (if (>= (- (Variables|Default|GetMaxStackSize) (CallFunction|-GetAmountatIndex (LocalVariables|GetLocalTo))) (CallFunction|-GetAmountatIndex (LocalVariables|GetLocalFrom)))
      (Utilities|Array|SetArrayElem (Variables|Default|GetSlots) (LocalVariables|GetLocalTo) (Utilities|Struct|Makes_InventorySlot (LocalVariables|GetLocalClass) (+ (CallFunction|-GetAmountatIndex (LocalVariables|GetLocalFrom)) (CallFunction|-GetAmountatIndex (LocalVariables|GetLocalTo)))))
      (Utilities|Array|SetArrayElem (Variables|Default|GetSlots) (LocalVariables|GetLocalFrom) (Utilities|Struct|Makes_InventorySlot 0 0))
      (else
        (Utilities|Array|SetArrayElem (Variables|Default|GetSlots) (LocalVariables|GetLocalFrom) (Utilities|Struct|Makes_InventorySlot (LocalVariables|GetLocalClass) (- (CallFunction|-GetAmountatIndex (LocalVariables|GetLocalFrom)) (- (Variables|Default|GetMaxStackSize) (CallFunction|-GetAmountatIndex (LocalVariables|GetLocalTo))))))
        (Utilities|Array|SetArrayElem (Variables|Default|GetSlots) (LocalVariables|GetLocalTo) (Utilities|Struct|Makes_InventorySlot (LocalVariables|GetLocalClass) (Variables|Default|GetMaxStackSize)))))
    ;[1 1 1] Два раза, т.к. у нас два слота
    (CallFunction|UpdateSlotatIndex (LocalVariables|GetLocalFrom))
    (CallFunction|UpdateSlotatIndex (LocalVariables|GetLocalTo))
    (return true)
    (else
      (return false))))

(fn -SplitStacktoIndex
  (params (FromIndex :type Integer) (ToIndex :type Integer) (Amount :type Integer))
  (LocalVariables|SetLocalFrom FromIndex)
  (LocalVariables|SetLocalTo ToIndex)
  (LocalVariables|SetLocalAmount Amount)
  (if (Math|Boolean|ANDBoolean (CallFunction|-IsSlotEmpty? (LocalVariables|GetLocalTo)) (not (CallFunction|-IsSlotEmpty? (LocalVariables|GetLocalFrom))) (.CanBeStacked (Utilities|Struct|Breaks_ItemInfo (.ItemInfo (CallFunction|-GetItemInfoatIndex (LocalVariables|GetLocalFrom))))) (> (.Amount (CallFunction|-GetItemInfoatIndex (LocalVariables|GetLocalFrom))) 1) (> (.Amount (CallFunction|-GetItemInfoatIndex (LocalVariables|GetLocalFrom))) (LocalVariables|GetLocalAmount)))
    (LocalVariables|SetLocalClass (.itemclass (Utilities|Array|Get(acopy) (Variables|Default|GetSlots) (LocalVariables|GetLocalFrom))))
    (Utilities|Array|SetArrayElem (Variables|Default|GetSlots) (LocalVariables|GetLocalFrom) (Utilities|Struct|Makes_InventorySlot (LocalVariables|GetLocalClass) (- (.amount (Utilities|Array|Get(acopy) (Variables|Default|GetSlots) (LocalVariables|GetLocalFrom))) (LocalVariables|GetLocalAmount))))
    (Utilities|Array|SetArrayElem (Variables|Default|GetSlots) (LocalVariables|GetLocalTo) (Utilities|Struct|Makes_InventorySlot (LocalVariables|GetLocalClass) (LocalVariables|GetLocalAmount)))
    (CallFunction|UpdateSlotatIndex (LocalVariables|GetLocalFrom))
    (CallFunction|UpdateSlotatIndex (LocalVariables|GetLocalTo))
    (return true)
    (else
      (return false))))

(fn -ShowObtainedItem
  (params (ItemClass :type BP%20Master%20Item%20Class%20Reference) (Amount :type Integer))
  (bind _mainwidget (Variables|Default|GetMainWidget))
  (if (Variables|Default|GetShowObtainedMessage?)
    (Utilities|IsValid _mainwidget
      (:Is%20Valid
        (Default|-AddItemtoObtainedQueue _mainwidget ItemClass Amount)
        (return true))
      (:Is%20Not%20Valid
        _)))
  (return false))

(fn -AddItem(Internal)
  (params (ItemClass :type BP%20Master%20Item%20Class%20Reference) (Amount :type Integer))
  (bind _slots (Variables|Default|GetSlots))
  (LocalVariables|SetLocalItemClass ItemClass)
  (LocalVariables|SetLocalAmount Amount)
  ;[1 1 1] Если не стакается
  (if (.CanBeStacked (Utilities|Struct|Breaks_ItemInfo (.ItemInfo (Utilities|GetClassDefaults ItemClass))))
    (bind (_sucess_ _index) (CallFunction|-SearchFreeStack (LocalVariables|GetLocalItemClass)))
    (if _sucess_
      (LocalVariables|SetLocalFoundIndex _index)
      (if (> (+ (.Amount (Utilities|Struct|Breaks_InventorySlot (Utilities|Array|Get(acopy) (Variables|Default|GetSlots) (LocalVariables|GetLocalFoundIndex)))) (LocalVariables|GetLocalAmount)) (Variables|Default|GetMaxStackSize))
        (LocalVariables|SetLocalAmount (- (+ (.Amount (Utilities|Struct|Breaks_InventorySlot (Utilities|Array|Get(acopy) (Variables|Default|GetSlots) (LocalVariables|GetLocalFoundIndex)))) (LocalVariables|GetLocalAmount)) (LocalVariables|GetLocalAmount)))
        (Utilities|Array|SetArrayElem _slots (LocalVariables|GetLocalFoundIndex) (Utilities|Struct|Makes_InventorySlot (LocalVariables|GetLocalItemClass) (Variables|Default|GetMaxStackSize)))
        (CallFunction|UpdateSlotatIndex (LocalVariables|GetLocalFoundIndex))
        (bind _rest (CallFunction|-AddItem(Internal) (LocalVariables|GetLocalItemClass) (LocalVariables|GetLocalAmount)))
        (return true _rest)
        (else
          (Utilities|Array|SetArrayElem _slots (LocalVariables|GetLocalFoundIndex) (Utilities|Struct|Makes_InventorySlot (LocalVariables|GetLocalItemClass) (+ (.Amount (Utilities|Struct|Breaks_InventorySlot (Utilities|Array|Get(acopy) (Variables|Default|GetSlots) (LocalVariables|GetLocalFoundIndex)))) (LocalVariables|GetLocalAmount))))
          (CallFunction|UpdateSlotatIndex (LocalVariables|GetLocalFoundIndex))
          (return true 0)))
      (else
        (bind (_success_ _index_2) (CallFunction|-SearchEmptySlot))
        (if _success_
          (bind _output_get (LocalVariables|SetLocalFoundIndex _index_2))
          (if (> (LocalVariables|GetLocalAmount) (Variables|Default|GetMaxStackSize))
            (Utilities|Array|SetArrayElem (Variables|Default|GetSlots) _output_get (Utilities|Struct|Makes_InventorySlot (LocalVariables|GetLocalItemClass) (Variables|Default|GetMaxStackSize)))
            (CallFunction|UpdateSlotatIndex (LocalVariables|GetLocalFoundIndex))
            (bind (_success__2 _rest_2) (CallFunction|-AddItem(Internal) (LocalVariables|GetLocalItemClass) (- (LocalVariables|GetLocalAmount) (Variables|Default|GetMaxStackSize))))
            (return _success__2 _rest_2)
            (else
              (Utilities|Array|SetArrayElem (Variables|Default|GetSlots) (LocalVariables|GetLocalFoundIndex) (Utilities|Struct|Makes_InventorySlot (LocalVariables|GetLocalItemClass) (LocalVariables|GetLocalAmount)))
              (CallFunction|UpdateSlotatIndex (LocalVariables|GetLocalFoundIndex))
              (return true 0)))
          (else
            (return false (LocalVariables|GetLocalAmount))))))
    (else
      (bind (_success__3 _index_3) (CallFunction|-SearchEmptySlot))
      (if _success__3
        (bind _output_get_2 (LocalVariables|SetLocalFoundIndex _index_3))
        (Utilities|Array|SetArrayElem (Variables|Default|GetSlots) _output_get_2 (Utilities|Struct|Makes_InventorySlot (LocalVariables|GetLocalItemClass) 1))
        (CallFunction|UpdateSlotatIndex (LocalVariables|GetLocalFoundIndex))
        (if (> (LocalVariables|GetLocalAmount) 1)
          (bind (_success__4 _rest_3) (CallFunction|-AddItem(Internal) (LocalVariables|GetLocalItemClass) (- (LocalVariables|GetLocalAmount) 1)))
          (return _success__4 _rest_3)
          (else
            (return true 0)))
        (else
          (return false (LocalVariables|GetLocalAmount)))))))

(fn -SpawnItemsClassinWorld
  (params (ItemClass :type BP%20Master%20Item%20Class%20Reference) (Amount :type Integer))
  (bind _topdowncharref (Variables|Default|GetTopDownCharRef))
  (bind _topdowncharref_2 (Variables|Default|GetTopDownCharRef))
  (bind _capsulecomponent (Variables|/Script/Engine.Character|GetCapsuleComponent _topdowncharref))
  (bind _capsulecomponent_2 (Variables|/Script/Engine.Character|GetCapsuleComponent _topdowncharref_2))
  (bind _returnvalue (Transformation|GetWorldLocation _capsulecomponent))
  (LocalVariables|SetLocal_ItemClass ItemClass)
  (LocalVariables|SetLocal_Amount Amount)
  ;[1 1 1] Вращать персонажа и искать свободное место
  (Utilities|FlowControl|ForLoopwithBreak 0 360 :!label _label
    (:LoopBody
      (bind _returnvalue_2 (Collision|LineTraceByChannel _returnvalue (+ _returnvalue (* (Math|Vector|GetForwardVector _capsulecomponent) (Variables|Default|GetDistaceSpawnItem))) "TraceTypeQuery1" false 0 "None" true "(R=1.000000,G=0.000000,B=0.000000,A=0.000000)" "(R=0.000000,G=1.000000,B=0.000000,A=0.000000)"))
      (if (not _returnvalue_2)
        (Game|SpawnActorfromClass "/Game/BainProject/InventorySystem/Blueprints/ItemClasses/BP_PickUpActor.BP_PickUpActor_C" (Math|Transform|MakeTransform (+ (* (Math|Vector|GetForwardVector _capsulecomponent_2) (Variables|Default|GetDistaceSpawnItem)) (Transformation|GetWorldLocation _capsulecomponent_2)) (.Rotation (Math|Transform|BreakTransform (.WorldView (Utilities|Struct|Breaks_ItemInfo (.ItemInfo (Utilities|GetClassDefaults (LocalVariables|GetLocal_ItemClass))))))) (.Scale (Math|Transform|BreakTransform (.WorldView (Utilities|Struct|Breaks_ItemInfo (.ItemInfo (Utilities|GetClassDefaults (LocalVariables|GetLocal_ItemClass)))))))) "Undefined" 0 (LocalVariables|GetLocal_ItemClass) (LocalVariables|GetLocal_Amount) 0)
        ;[1 1 1] Для поиска места для спавна предмета
        (LocalVariables|SetLocal_Drop true)
        (goto _label Break)))
    (:Completed
      (if (LocalVariables|GetLocal_Drop)
        (return)
        (else
          (Game|SpawnActorfromClass "/Game/BainProject/InventorySystem/Blueprints/ItemClasses/BP_PickUpActor.BP_PickUpActor_C" (Math|Transform|MakeTransform (Transformation|GetWorldLocation (Variables|/Script/Engine.Character|GetCapsuleComponent (Variables|Default|GetTopDownCharRef))) (.Rotation (Math|Transform|BreakTransform (.WorldView (Utilities|Struct|Breaks_ItemInfo (.ItemInfo (Utilities|GetClassDefaults (LocalVariables|GetLocal_ItemClass))))))) (.Scale (Math|Transform|BreakTransform (.WorldView (Utilities|Struct|Breaks_ItemInfo (.ItemInfo (Utilities|GetClassDefaults (LocalVariables|GetLocal_ItemClass)))))))) "Undefined" 0 (LocalVariables|GetLocal_ItemClass) (LocalVariables|GetLocal_Amount) 0)
          (return))))))