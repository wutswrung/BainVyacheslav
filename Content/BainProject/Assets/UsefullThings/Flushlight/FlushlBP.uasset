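; FlushlBP is an actor that shows interaction prompts and a closed/open indicator tied to a keypad door.
; Box overlaps toggle the PressE prompt, or OpenClose once the code is valid.
; Tick polls whether the player's InteractableActor is the first Door_WithKeyPad found in the level.
; When that door reports a valid code, it latches CodeIsValid, swaps PlaneClosed for PlaneOpen and hides PressE.
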(event OnComponentBeginOverlap(Box)
  (params (OverlappedComponent :type Primitive%20Component%20Object%20Reference) (OtherActor :type Actor%20Object%20Reference) (OtherComp :type Primitive%20Component%20Object%20Reference) (OtherBodyIndex :type Integer) (bFromSweep :type Boolean) (SweepResult :type Hit%20Result%20Structure%20%28by%20ref%29))
  (if (Variables|Default|GetCodeIsValid)
    (Rendering|SetVisibility (Variables|Default|GetOpenClose) true false)
    (else
      (Rendering|SetVisibility (Variables|Default|GetPressE) true false))))

(event OnComponentEndOverlap(Box)
  (params (OverlappedComponent :type Primitive%20Component%20Object%20Reference) (OtherActor :type Actor%20Object%20Reference) (OtherComp :type Primitive%20Component%20Object%20Reference) (OtherBodyIndex :type Integer))
  (if (Variables|Default|GetCodeIsValid)
    (Rendering|SetVisibility (Variables|Default|GetOpenClose) false false)
    (else
      (Rendering|SetVisibility (Variables|Default|GetPressE) false false))))

(event EventBeginPlay)

(event Collision|EventActorBeginOverlap
  (params (OtherActor :type Actor%20Object%20Reference)))

(event EventTick
  (params (DeltaSeconds :type Float%20%28single-precision%29))
  (bind _asmain_character (Utilities|Casting|CastToMainCharacter (Game|GetPlayerCharacter 0)))
  (bind _outactors (Actor|GetAllActorsOfClass "/Game/BainProject/Interaction/CodeDoor/Door_WithKeyPad.Door_WithKeyPad_C"))
  (if (== (Utilities|Array|Get(acopy) _outactors) (Variables|/Game/BainProject/Characters/MainCharacter.MainCharacter_C|GetInteractableActor _asmain_character))
    (bind _asdoor_with_key_pad (Utilities|Casting|CastToDoor_WithKeyPad (Variables|/Game/BainProject/Characters/MainCharacter.MainCharacter_C|GetInteractableActor _asmain_character)))
    (if (Variables|/Game/BainProject/Interaction/CodeDoor/Door_WithKeyPad.Door_WithKeyPad_C|GetValidCodeEntered _asdoor_with_key_pad)
      (Rendering|SetVisibility (Variables|Default|GetPlaneClosed) false false)
      (Rendering|SetVisibility (Variables|Default|GetPlaneOpen) true false)
      (Variables|Default|SetCodeIsValid true)
      (Rendering|SetVisibility (Variables|Default|GetPressE) false false))))

(fn ConstructionScript)